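; JohnsonBp is the Johnson player character in LostDog, handling movement, camera turning, pausing and a timed posting state.
; Axis inputs move the character relative to control rotation yaw and turn the controller horizontally.
; The E key raises an IsPosting flag, then clears it after a short delay.
; The Pause action toggles game pause, creating a PauseHUD widget on pause without removing it on unpause.
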(event `Key|E`
  (params (Key :type "Key Structure"))
  (:`Pressed`
    (set `self.IsPosting?` true)
    (`KismetSystemLibrary.Delay` 2.0)
    (set `self.IsPosting?` false)))

(event `InputAction|Pause`
  (params (Key :type "Key Structure"))
  ;[1 1 1] Pause
  (:`Pressed`
    (if (`self.IsPaused`)
      (set `self.IsPaused` false)
      (`GameplayStatics.SetGamePaused` false)
      (else
        (bind _returnvalue (`|CreateWidget` "/Game/LostDog/Maps/MainMenu/PauseHUD.PauseHUD_C"))
        (`UserWidget.AddToViewport` _returnvalue 0)
        (set `self.IsPaused` true)
        (`GameplayStatics.SetGamePaused` true)))))

(event `InputAxis|MoveForward`
  (params (AxisValue :type "Float (single-precision)"))
  (bind (_returnvalue_roll _returnvalue_pitch _returnvalue_yaw) (`KismetMathLibrary.BreakRotator` (`self.GetControlRotation`)))
  ;[1 1 1] Movement
  (`self.AddMovementInput` (`KismetMathLibrary.GetForwardVector` (`KismetMathLibrary.MakeRotator` 0.0 0.0 _returnvalue_yaw)) AxisValue))

(event `InputAxis|MoveRight`
  (params (AxisValue :type "Float (single-precision)"))
  (bind (_returnvalue_roll _returnvalue_pitch _returnvalue_yaw) (`KismetMathLibrary.BreakRotator` (`self.GetControlRotation`)))
  ;[1 1 1] Movement
  (`self.AddMovementInput` (`KismetMathLibrary.GetRightVector` (`KismetMathLibrary.MakeRotator` 0.0 0.0 _returnvalue_yaw)) AxisValue))

(event `InputAxis|Turn`
  (params (AxisValue :type "Float (single-precision)"))
  ;[1 1 1] Camera rotation
  (`self.AddControllerYawInput` AxisValue))

(fn `UserConstructionScript`)